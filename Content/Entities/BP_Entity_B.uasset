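; BP_Entity_B is an entity Blueprint that shows its current state through the color of its sphere mesh.
; On BeginPlay it creates a dynamic material instance from the sphere's material and assigns it back to the mesh.
; Events for normal, hit, attack and dead states each set that material's Color parameter, with only the normal-state event checking the instance is valid first.
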(event `self.ReceiveBeginPlay`
  (bind _sphere (`self.Sphere`))
  (bind _returnvalue (`PrimitiveComponent.CreateDynamicMaterialInstance` _sphere 0 (`PrimitiveComponent.GetMaterial` _sphere 0) "None"))
  (bind _output_get (set `self.DynamicMaterial` _returnvalue))
  (`PrimitiveComponent.SetMaterial` (`self.Sphere`) 0 _output_get))

(event `self.OnNormalState`
  (bind _dynamicmaterial (`self.DynamicMaterial`))
  (`/Engine/EditorBlueprintResources/StandardMacros.IsValid` _dynamicmaterial
    (:`Is Valid`
      (`MaterialInstanceDynamic.SetVectorParameterValue` _dynamicmaterial "Color" (struct :`R` 0.003254 :`B` 1.0 :`A` 1.0)))))

(event `self.OnReceiveHit`
  (`MaterialInstanceDynamic.SetVectorParameterValue` (`self.DynamicMaterial`) "Color" (struct :`R` 1.0 :`B` 0.788176 :`A` 1.0)))

(event `self.OnDeadState`
  (`MaterialInstanceDynamic.SetVectorParameterValue` (`self.DynamicMaterial`) "Color" (struct :`A` 1.0)))

(event `self.OnAttackState`
  (`MaterialInstanceDynamic.SetVectorParameterValue` (`self.DynamicMaterial`) "Color" (struct :`G` 0.85423 :`B` 1.0 :`A` 1.0)))

(fn `UserConstructionScript`)